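; Base 2D side-view character Blueprint that handles left/right movement, walking and jumping through Enhanced Input.
; Move inputs set a direction value, add movement along world X and flip the sprite's yaw to face that way; movement and walk respect an input-disable flag.
; Walk lowers max speed and immediately clamps excess X velocity, restoring run speed on completion.
; Jump, which ignores that flag, also sends a state message to the AnimInstance.
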(event `self.ReceiveBeginPlay`)

(event `EnhancedInput|/Game/BluePrint/InputAction/IA_MoveRight`
  (params (ActionValue :type Boolean) (ElapsedSeconds :type "Float (double-precision)") (TriggeredSeconds :type "Float (double-precision)") (InputAction :type "InputAction Object Reference" :default "/Game/BluePrint/InputAction/IA_MoveRight.IA_MoveRight"))
  ; 移动
  (:`Triggered`
    ; 是否禁用输入
    (if (not (`self.bIsDisableInput`))
      ; 根据输入设置角色朝向
      (set `self.FMoveForward` 1.0)
      ; 根据朝向，沿X轴移动
      (`self.AddMovementInput` (1.0 0.0 0.0) (`self.FMoveForward`) :!label _label)
      (`self.SetTheCharacterDirection`))))

(event `EnhancedInput|/Game/BluePrint/InputAction/IA_MoveLeft`
  (params (ActionValue :type Boolean) (ElapsedSeconds :type "Float (double-precision)") (TriggeredSeconds :type "Float (double-precision)") (InputAction :type "InputAction Object Reference" :default "/Game/BluePrint/InputAction/IA_MoveLeft.IA_MoveLeft"))
  ; 移动
  (:`Triggered`
    ; 是否禁用输入
    (if (not (`self.bIsDisableInput`))
      ; 根据输入设置角色朝向
      (set `self.FMoveForward` -1.0)
      (goto _label))))

(event `EnhancedInput|/Game/BluePrint/InputAction/IA_Walk`
  (params (ActionValue :type Boolean) (ElapsedSeconds :type "Float (double-precision)") (TriggeredSeconds :type "Float (double-precision)") (InputAction :type "InputAction Object Reference" :default "/Game/BluePrint/InputAction/IA_Walk.IA_Walk"))
  (bind _charactermovement (`self.CharacterMovement`))
  ; 设置是否为行走
  (:`Triggered`
    ; 是否禁用输入
    (if (not (`self.bIsDisableInput`))
      ; 获取移动组件
      ; 设置移动速度
      (set `CharacterMovementComponent.MaxWalkSpeed` (`self.fMaxWalkSpeed`) _charactermovement)
      (`self.SetCharacterMovementVelocity` _charactermovement)))
  (:`Completed`
    (set `CharacterMovementComponent.MaxWalkSpeed` (`self.fMaxRunSpeed`) (`self.CharacterMovement`))))

(event `EnhancedInput|/Game/BluePrint/InputAction/IA_Jump`
  (params (ActionValue :type Boolean) (ElapsedSeconds :type "Float (double-precision)") (TriggeredSeconds :type "Float (double-precision)") (InputAction :type "InputAction Object Reference" :default "/Game/BluePrint/InputAction/IA_Jump.IA_Jump"))
  ; 空格跳跃
  (:`Triggered`
    (`self.Jump`)
    (message `/Game/BluePrint/Character/C_Xia_101/C_Xia_CharState_BPI.CharState` (`self.GetAnimInstance`) "NewEnumerator3")))

(event `self.ReceiveTick`
  (params (DeltaSeconds :type "Float (single-precision)")))

(fn `SetCharacterMovementVelocity`
  (params (CharacterMovement :type "MovementComponent Object Reference"))
  (bind (_velocity_x _velocity_y _velocity_z) (`KismetMathLibrary.BreakVector` (`MovementComponent.Velocity` CharacterMovement)))
  (if (> (`KismetMathLibrary.Abs` _velocity_x) (`self.fMaxWalkSpeed`))
    (set `MovementComponent.Velocity` (`KismetMathLibrary.MakeVector` (* (`self.fMoveForward`) (`self.fMaxWalkSpeed`)) _velocity_y _velocity_z) CharacterMovement)
    (else
      (set `MovementComponent.Velocity` (`KismetMathLibrary.MakeVector` _velocity_x _velocity_y _velocity_z) CharacterMovement))))

(fn `SetTheCharacterDirection`
  (bind _sprite (`self.Sprite`))
  (bind _location (.location (`SceneComponent.GetRelativeTransform` _sprite)))
  (bind _scale (.scale (`SceneComponent.GetRelativeTransform` _sprite)))
  (bind _roll (.roll (.rotation (`SceneComponent.GetRelativeTransform` _sprite))))
  (bind _pitch (.pitch (.rotation (`SceneComponent.GetRelativeTransform` _sprite))))
  (if (== (`self.FMoveForward`) 1.0)
    (`SceneComponent.K2_SetRelativeTransform` _sprite (`KismetMathLibrary.MakeTransform` _location (`KismetMathLibrary.MakeRotator` _roll _pitch 180.0) _scale) false false)
    (else
      (`SceneComponent.K2_SetRelativeTransform` _sprite (`KismetMathLibrary.MakeTransform` _location (`KismetMathLibrary.MakeRotator` _roll _pitch) _scale) false false))))

(fn `UserConstructionScript`)